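; BP_collectible is an interactable actor whose Cube mesh toggles visibility on player input; despite the name, no pickup logic is present.
; The cube starts hidden, and Box overlap events set PlayerInzone and enable or disable the actor's input for player controller 0, without checking which actor overlapped.
; E and the gamepad left face button each drive a separate FlipFlop to show or hide the cube, so their toggle states can drift apart.
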(event OnComponentBeginOverlap(Box)
  (params (OtherActor :type Actor%20Object%20Reference) (OtherComp :type Primitive%20Component%20Object%20Reference) (OtherBodyIndex :type Integer) (bFromSweep :type Boolean) (SweepResult :type Hit%20Result%20Structure%20%28by%20ref%29))
  (Variables|Default|SetPlayer_inzone true)
  (Input|EnableInput (Game|GetPlayerController 0)))

(event OnComponentEndOverlap(Box)
  (params (OtherActor :type Actor%20Object%20Reference) (OtherComp :type Primitive%20Component%20Object%20Reference) (OtherBodyIndex :type Integer))
  (Variables|Default|SetPlayer_inzone false)
  (Input|DisableInput (Game|GetPlayerController 0)))

(event EventBeginPlay
  (Rendering|SetVisibility (Variables|Default|GetCube) false false))

(event EventActorBeginOverlap
  (params (OtherActor :type Actor%20Object%20Reference)))

(event EventTick
  (params (DeltaSeconds :type Float%20%28single-precision%29)))

(event Input|GamepadEvents|GamepadFaceButtonLeft
  (params (Key :type Key%20Structure :default "AnyKey"))
  (:Pressed
    (if (Variables|Default|GetPlayer_inzone)
      (Utilities|FlowControl|FlipFlop
        (:A
          (Rendering|SetVisibility (Variables|Default|GetCube) true false))
        (:B
          (Rendering|SetVisibility (Variables|Default|GetCube) false false))))))

(event Input|KeyboardEvents|E
  (params (Key :type Key%20Structure :default "AnyKey"))
  (:Pressed
    (if (Variables|Default|GetPlayer_inzone)
      (Utilities|FlowControl|FlipFlop
        (:A
          (Rendering|SetVisibility (Variables|Default|GetCube) true false))
        (:B
          (Rendering|SetVisibility (Variables|Default|GetCube) false false))))))

(fn ConstructionScript)