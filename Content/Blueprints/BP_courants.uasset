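; Spline-driven current actor (courants) that lays a strip of spline meshes along its path.
; Construction adds a manually attached mesh per Spacing step, using world-space spline points with direction tangents scaled by Smoothness.
; Each segment gets a dynamic M_courant material, stored in SplineMaterials and sharing one random wind variation.
; BeginPlay binds to OnChangeStreamType, but the handler's loop is empty: its wind and type parameter setters are disconnected.
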(event Custom|OnChangeStreamType_Event_0
  (params (matWind :type Float%20%28single-precision%29) (matType :type Float%20%28single-precision%29))
  (for _array_element (Variables|Default|GetSplineMaterials)
    _))

(event EventBeginPlay
  (EventDispatchers|AssignOnChangeStreamType (delegate Custom|OnChangeStreamType_Event_0)))

(event EventActorBeginOverlap
  (params (OtherActor :type Actor%20Object%20Reference)))

(event EventTick
  (params (DeltaSeconds :type Float%20%28single-precision%29)))

(fn ConstructionScript
  (bind _smoothness (Variables|Default|GetSmoothness))
  (bind _spline (Variables|Default|GetSpline))
  (bind _spacing (Variables|Default|GetSpacing))
  (Variables|Default|SetVariation (Math|Random|RandomFloatinRange 0.0 5.0))
  (for _index (range 0 (.ReturnValue (Math|Float|Division(WholeandRemainder) (Spline|GetSplineLength _spline) _spacing)))
    (bind _returnvalue (AddComponent|AddSplineMeshComponent true))
    (Components|StaticMesh|SetStaticMesh _returnvalue (Variables|Default|Getmesh))
    (bind _returnvalue_2 (Rendering|Material|CreateDynamicMaterialInstance "/Game/Material/Master/M_courant.M_courant" :!class /Script/Engine.KismetMaterialLibrary))
    (Utilities|Array|Add (Variables|Default|GetSplineMaterials) _returnvalue_2)
    (bind _output_get (Variables|Default|Setmaterial _returnvalue_2))
    (Rendering|Material|SetMaterial _returnvalue 0 _output_get)
    (Rendering|Material|SetScalarParameterValue _returnvalue_2 "wind_variation" (Variables|Default|GetVariation) :!class /Script/Engine.MaterialInstanceDynamic)
    (SplineMesh|SetStartandEnd _returnvalue (Spline|GetLocationatDistanceAlongSpline _spline (* _index _spacing) "World") (* (Spline|GetDirectionatDistanceAlongSpline _spline (* _index _spacing) "World") _smoothness) (Spline|GetLocationatDistanceAlongSpline _spline (+ (* _index _spacing) _spacing) "World") (* (Spline|GetDirectionatDistanceAlongSpline _spline (+ (* _index _spacing) _spacing) "World") _smoothness) :!class /Script/Engine.SplineMeshComponent)))