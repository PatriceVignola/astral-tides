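; Project Luna game mode that swaps streamed levels when its OnLevelStreamLoad event fires.
; It unloads each level in UnloadList one at a time, then loads and shows each in LoadList without blocking.
; Index counters loop back through the latent stream nodes, with each list's first entry processed before any length check.
; Once the last load finishes, it calls OnLevelLoaded with the level number and load origin.
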(event Custom|OnLevelStreamLoad_Event_0
  (params (levelNumber :type Integer) (loadOrigin :type Integer) (loadList :type Array%20of%20Strings) (unloadList :type Array%20of%20Strings))
  (Game|UnloadStreamLevel(byName) (Utilities|String|StringToName (Utilities|Array|Get(acopy) unloadList (Variables|Default|GetUnloadIndex))) :!label _label)
  (bind _result (Math|Integer|IncrementInt (Variables|Default|GetUnloadIndex))
    (:%20%20
      (if (== (Utilities|Array|Length unloadList) _result)
        (Variables|Default|SetUnloadIndex 0)
        (Game|LoadStreamLevel(byName) (Utilities|String|StringToName (Utilities|Array|Get(acopy) loadList (Variables|Default|GetLoadIndex))) true :!label _label_2)
        (bind _result_2 (Math|Integer|IncrementInt (Variables|Default|GetLoadIndex))
          (:%20%20
            (if (== (Utilities|Array|Length loadList) _result_2)
              (Class|ProjectLunaGameMode|OnLevelLoaded levelNumber loadOrigin)
              (Variables|Default|SetLoadIndex 0)
              (else
                (goto _label_2)))))
        (else
          (goto _label))))))

(event EventBeginPlay
  (EventDispatchers|AssignOnLevelStreamLoad (delegate Custom|OnLevelStreamLoad_Event_0)))

(event EventTick
  (params (DeltaSeconds :type Float%20%28single-precision%29)))

(fn ConstructionScript)