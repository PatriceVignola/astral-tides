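; Wolf character Blueprint that adds Wwise audio, a particle component and foot IK support.
; On BeginPlay it binds events to post footstep, ice block drag and death splash sounds, and forwards stream and orca attenuation to BP_SoundManager.
; Construction passes the wolf to particles as ParticleLocation and derives the IK trace distance from scaled capsule half-height.
; IKFootTrace line-traces down at a foot socket and returns a scale-corrected ground offset.
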(event Custom|OnFootStep_Event_0
  (Class|AkComponent|PostAkEvent (stale EventBeginPlay _returnvalue) "/Game/Sounds/Wwise/Events/Wolf_FS.Wolf_FS"))

(event Custom|OnOrquaSoundAttenuation_Event_0
  (params (ratio :type Float%20%28single-precision%29))
  (Default|AttenuateOrqua (Variables|Default|GetSoundManager) ratio))

(event Custom|OnDied_Event_0
  (Class|AkComponent|PostAkEvent (Variables|Default|GetAKComponent) "/Game/Sounds/Wwise/Events/Wolf_WaterSplash.Wolf_WaterSplash"))

(event Custom|OnStartedPushingBlock_Event_0
  (Class|AkComponent|PostAkEvent (Variables|Default|GetAKComponent) "/Game/Sounds/Wwise/Events/Icecube_Drag.Icecube_Drag"))

(event Custom|OnStoppedPushingBlock_Event_0
  (Class|AkComponent|PostAkEvent (Variables|Default|GetAKComponent) "/Game/Sounds/Wwise/Events/Icecube_Stop.Icecube_Stop"))

(event Custom|OnStreamAttenuation_Event_0
  (params (ratio :type Float%20%28single-precision%29))
  (Default|AttenuateStream (Variables|Default|GetSoundManager) ratio))

(event EventBeginPlay
  (bind _outactors (Actor|GetAllActorsOfClass "/Game/Blueprints/BP_SoundManager.BP_SoundManager_C"))
  (for _array_element _outactors
    (Variables|Default|SetSoundManager _array_element))
  (bind _returnvalue (AddComponent|AddAkComponent false))
  (Variables|Default|SetAKComponent _returnvalue)
  (EventDispatchers|AssignOnFootStep (delegate Custom|OnFootStep_Event_0))
  (EventDispatchers|AssignOnStreamAttenuation (delegate Custom|OnStreamAttenuation_Event_0))
  (EventDispatchers|AssignOnOrquaSoundAttenuation (delegate Custom|OnOrquaSoundAttenuation_Event_0))
  (EventDispatchers|AssignOnDied (delegate Custom|OnDied_Event_0))
  (EventDispatchers|AssignOnStartedPushingBlock (delegate Custom|OnStartedPushingBlock_Event_0))
  (EventDispatchers|AssignOnStoppedPushingBlock (delegate Custom|OnStoppedPushingBlock_Event_0)))

(fn ConstructionScript
  (bind _returnvalue (AddComponent|AddParticleSystemComponent false))
  (Effects|Components|ParticleSystem|SetActorParameter _returnvalue "ParticleLocation" self)
  (bind _output_get (Variables|Default|SetScale (.Z (Math|Vector|BreakVector (.Scale (Math|Transform|BreakTransform (Transformation|GetActorTransform)))))))
  (Variables|Default|SetIKTraceDistance (* (Components|Capsule|GetUnscaledCapsuleHalfHeight (Variables|Default|GetCapsuleComponent)) _output_get)))

(fn IKFootTrace
  (params (TraceDIstance :type Float%20%28single-precision%29) (Socket :type Name))
  (bind _returnvalue (Transformation|GetActorLocation))
  (bind _mesh (Variables|Character|GetMesh))
  (bind _returnvalue_2 (Transformation|GetSocketLocation _mesh Socket))
  (bind _z (Math|Vector|BreakVector _returnvalue))
  (bind (_x _y) (Math|Vector|BreakVector _returnvalue_2))
  (bind _returnvalue_3 (- _z TraceDIstance))
  (bind _returnvalue_4 (Math|Vector|MakeVector _x _y _returnvalue_3))
  ;[1 1 1] Trace from Socket Locations to bottom of character
  (bind (_outhit _returnvalue_5) (Collision|LineTraceByChannel (Math|Vector|MakeVector _x _y _z) _returnvalue_4 "TraceTypeQuery1" true 0 "None"))
  ;[1 1 1] If it hits something it will calculate difference and return it as an offset
  (return (Math|Float|SelectFloat (/ (Math|Vector|VectorLength (- _returnvalue_4 (.Location (Collision|BreakHitResult _outhit)))) (Variables|Default|GetScale)) 0.0 _returnvalue_5)))