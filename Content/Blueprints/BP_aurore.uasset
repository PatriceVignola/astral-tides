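; BP_aurore is an aurora effect actor that lays a ribbon of plane meshes along an editable spline.
; Its construction script adds a spline mesh every Spacing units, bending each with world-space positions and Smoothness-scaled tangents from the spline.
; Each segment gets its own M_Aurore dynamic material, all sharing one random value rolled per construction run.
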(fn ConstructionScript
  (bind _smoothness (Variables|Default|GetSmoothness))
  (bind _spline (Variables|Default|GetSpline))
  (bind _spacing (Variables|Default|GetSpacing))
  (Variables|Default|SetRandom_set (Math|Random|RandomFloatinRange 0.0 5e+01))
  (for _index (range 0 (.ReturnValue (Math|Float|Division(WholeandRemainder) (Spline|GetSplineLength _spline) _spacing)))
    (bind _returnvalue (AddComponent|AddSplineMeshComponent true))
    (Components|StaticMesh|SetStaticMesh _returnvalue "/Game/Assets/Autres/SM_plane_aurore.SM_plane_aurore")
    (bind _returnvalue_2 (Rendering|Material|CreateDynamicMaterialInstance "/Game/Material/Master/M_Aurore.M_Aurore" :!class /Script/Engine.KismetMaterialLibrary))
    (bind _output_get (Variables|Default|Setmaterial _returnvalue_2))
    (Rendering|Material|SetMaterial _returnvalue 0 _output_get)
    (Rendering|Material|SetScalarParameterValue _returnvalue_2 "RandomValue" (Variables|Default|GetRandom_set) :!class /Script/Engine.MaterialInstanceDynamic)
    (SplineMesh|SetStartandEnd _returnvalue (Spline|GetLocationatDistanceAlongSpline _spline (* _index _spacing) "World") (* (Spline|GetDirectionatDistanceAlongSpline _spline (* _index _spacing) "World") _smoothness) (Spline|GetLocationatDistanceAlongSpline _spline (+ (* _index _spacing) _spacing) "World") (* (Spline|GetDirectionatDistanceAlongSpline _spline (+ (* _index _spacing) _spacing) "World") _smoothness) :!class /Script/Engine.SplineMeshComponent)))