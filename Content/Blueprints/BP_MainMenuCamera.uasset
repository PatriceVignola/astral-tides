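; BP_MainMenuCamera is the main menu camera Blueprint, which here handles Wwise UI audio for menu navigation.
; On BeginPlay it adds an AkComponent, then binds handlers to its start game, next, previous, back and confirm option dispatchers.
; Each handler posts the matching UI Ak event on that component.
; The dispatchers are not triggered in this graph, and the construction script is empty.
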(event Custom|OnStartGame_Event_0
  (Class|AkComponent|PostAkEvent (Variables|Default|GetAKComponent) "/Game/Sounds/Wwise/Events/UI_startGame.UI_startGame"))

(event Custom|OnSelectNextOption_Event_0
  (Class|AkComponent|PostAkEvent (Variables|Default|GetAKComponent) "/Game/Sounds/Wwise/Events/UI_navigation_right.UI_navigation_right"))

(event Custom|OnSelectPrevOption_Event_0
  (Class|AkComponent|PostAkEvent (Variables|Default|GetAKComponent) "/Game/Sounds/Wwise/Events/UI_navigation_left.UI_navigation_left"))

(event Custom|OnBackOption_Event_0
  (Class|AkComponent|PostAkEvent (Variables|Default|GetAKComponent) "/Game/Sounds/Wwise/Events/UI_back.UI_back"))

(event Custom|OnConfirmOption_Event_0
  (Class|AkComponent|PostAkEvent (Variables|Default|GetAKComponent) "/Game/Sounds/Wwise/Events/UI_confirm.UI_confirm"))

(event EventActorBeginOverlap
  (params (OtherActor :type Actor%20Object%20Reference)))

(event EventTick
  (params (DeltaSeconds :type Float%20%28single-precision%29)))

(event EventBeginPlay
  (bind _returnvalue (AddComponent|AddAkComponent false))
  (Variables|Default|SetAKComponent _returnvalue)
  (Utilities|FlowControl|Sequence
    (:then_0
      (EventDispatchers|AssignOnStartGame (delegate Custom|OnStartGame_Event_0)))
    (:then_1
      (EventDispatchers|AssignOnSelectNextOption (delegate Custom|OnSelectNextOption_Event_0)))
    (:then_2
      (EventDispatchers|AssignOnSelectPrevOption (delegate Custom|OnSelectPrevOption_Event_0)))
    (:then_3
      (EventDispatchers|AssignOnBackOption (delegate Custom|OnBackOption_Event_0)))
    (:then_4
      (EventDispatchers|AssignOnConfirmOption (delegate Custom|OnConfirmOption_Event_0)))))

(fn ConstructionScript)