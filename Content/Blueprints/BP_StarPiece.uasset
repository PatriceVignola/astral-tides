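; BP_StarPiece is a star piece actor that floats and spins, and plays a sound when a wolf overlaps it.
; Tick keeps calling Play on a timeline, whose updates add a Z offset to the current location and a small yaw step.
; BeginPlay adds a Wwise Ak component, which posts Col_Star when a BP_Wolf or subclass overlaps.
; The overlap only triggers audio, with no pickup or destroy logic here.
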(event Collision|EventActorBeginOverlap
  (params (OtherActor :type Actor%20Object%20Reference))
  (if (Utilities|ClassIsChildOf (Utilities|GetClass OtherActor) "/Game/Blueprints/BP_Wolf.BP_Wolf_C")
    (Class|AkComponent|PostAkEvent (Variables|Default|GetAKComponent) "/Game/Sounds/Wwise/Events/Col_Star.Col_Star")))

(event EventBeginPlay
  (bind _returnvalue (AddComponent|AddAkComponent false))
  (Variables|Default|SetAKComponent _returnvalue))

(event EventActorBeginOverlap
  (params (OtherActor :type Actor%20Object%20Reference)))

(event EventTick
  (params (DeltaSeconds :type Float%20%28single-precision%29))
  (bind _returnvalue (Transformation|GetActorRotation))
  (bind _returnvalue_2 (Transformation|GetActorLocation))
  (bind (_roll _pitch _yaw) (Math|Rotator|BreakRotator _returnvalue))
  (bind (_x _y _z) (Math|Vector|BreakVector _returnvalue_2))
  (bind _z_pos (Timeline|Timeline_0 Play)
    (:Update
      (Transformation|SetActorLocationAndRotation (Math|Vector|MakeVector _x _y (+ _z _z_pos)) (Math|Rotator|MakeRotator _roll _pitch (+ _yaw 0.15))))))

(fn ConstructionScript)