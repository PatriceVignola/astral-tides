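; BP_SoundManager is an actor that drives the game's Wwise audio through a single AkComponent added at BeginPlay.
; BeginPlay sets initial RTPCs and the ice surface switch, posts the Gamestart event, then binds the howl start and stop delegates.
; Howl up and down callbacks start and stop the WaterUp and WaterDown events.
; AttenuateStream and AttenuateOrqua scale a ratio by 100 into the ice-cube and orc attenuation RTPCs.
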(event Custom|OnStartHowlUp_Event_0
  (Class|AkComponent|PostAkEvent (Variables|Default|GetAKComponent) "/Game/Sounds/Wwise/Events/WaterUp.WaterUp"))

(event Custom|OnStartHowlDown_Event_0
  (Class|AkComponent|PostAkEvent (Variables|Default|GetAKComponent) "/Game/Sounds/Wwise/Events/WaterDown.WaterDown"))

(event Custom|OnStopHowlUp_Event_0
  (Class|AkComponent|PostAkEvent (Variables|Default|GetAKComponent) "/Game/Sounds/Wwise/Events/WaterUp_Stop.WaterUp_Stop"))

(event Custom|OnStopHowlDown_Event_0
  (Class|AkComponent|PostAkEvent (Variables|Default|GetAKComponent) "/Game/Sounds/Wwise/Events/WaterDown_Stop.WaterDown_Stop"))

(event EventBeginPlay
  (bind _returnvalue (AddComponent|AddAkComponent false))
  (Variables|Default|SetAKComponent _returnvalue)
  (Utilities|FlowControl|Sequence
    (:then_0
      (Class|AkComponent|SetRTPCValue _returnvalue "Game_Altitude" 5e+01))
    (:then_1
      (Class|AkComponent|SetRTPCValue _returnvalue "Orc_Attenuation" 0.0))
    (:then_2
      (Class|AkComponent|SetRTPCValue _returnvalue "IcecubeMoving_Attenuation" 0.0))
    (:then_3
      (Class|AkComponent|SetSwitch _returnvalue "FS_Surface" "Ice"))
    (:then_4
      (Class|AkComponent|PostAkEvent _returnvalue "/Game/Sounds/Wwise/Events/Gamestart.Gamestart")
      (Utilities|FlowControl|Sequence
        (:then_0
          (EventDispatchers|AssignOnStartHowlUp (delegate Custom|OnStartHowlUp_Event_0)))
        (:then_1
          (EventDispatchers|AssignOnStartHowlDown (delegate Custom|OnStartHowlDown_Event_0)))
        (:then_2
          (EventDispatchers|AssignOnStopHowlUp (delegate Custom|OnStopHowlUp_Event_0)))
        (:then_3
          (EventDispatchers|AssignOnStopHowlDown (delegate Custom|OnStopHowlDown_Event_0)))))))

(event EventActorBeginOverlap
  (params (OtherActor :type Actor%20Object%20Reference)))

(event EventTick
  (params (DeltaSeconds :type Float%20%28single-precision%29)))

(fn ConstructionScript)

(fn AttenuateStream
  (params (ratio :type Float%20%28single-precision%29))
  (Class|AkComponent|SetRTPCValue (Variables|Default|GetAKComponent) "IcecubeMoving_Attenuation" (* ratio 1e+02)))

(fn AttenuateOrqua
  (params (ratio :type Float%20%28single-precision%29))
  (Class|AkComponent|SetRTPCValue (Variables|Default|GetAKComponent) "Orc_Attenuation" (* ratio 1e+02)))